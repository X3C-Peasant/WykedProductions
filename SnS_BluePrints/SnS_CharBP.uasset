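; SnS_CharBP is a player character Blueprint that handles look, movement, sprint, crouch and prone input.
; Movement follows zero-rotation world axes rather than control rotation, and is gated by DisableMovement.
; Sprint and crouch change walk speed, while FlipFlops toggle crouch and prone, each blocked by the other's flag.
; The stance flags are only ever set false here, and prone has no pose or speed logic.
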(event EventBeginPlay)

(event Collision|EventActorBeginOverlap
  (params (OtherActor :type Actor%20Object%20Reference)))

(event EventTick
  (params (DeltaSeconds :type Float%20%28single-precision%29)))

(event Input|ActionEvents|InputActionSprint
  (params (Key :type Key%20Structure))
  (bind _charactermovement (Variables|Character|GetCharacterMovement))
  (:Pressed
    (Variables|Default|SetSprintPressed false)
    (Variables|/Script/Engine.CharacterMovementComponent|SetMaxWalkSpeed _charactermovement 3.6e+02))
  (:Released
    (Variables|Default|SetSprintPressed false)
    (if (Variables|Default|GetCrouchPressed)
      (Variables|/Script/Engine.CharacterMovementComponent|SetMaxWalkSpeed _charactermovement 246.0)
      (else
        (Variables|/Script/Engine.CharacterMovementComponent|SetMaxWalkSpeed _charactermovement 198.0)))))

(event Input|ActionEvents|InputActionProne
  (params (Key :type Key%20Structure))
  (:Pressed
    (if (not (Variables|Default|GetCrouchPressed))
      (Utilities|FlowControl|FlipFlop
        (:A
          (Variables|Default|SetPronePressed false)
          (Variables|Default|SetDisableMovement false))
        (:B
          (Variables|Default|SetPronePressed false)
          (Utilities|FlowControl|Delay 0.2))))))

(event Input|ActionEvents|InputActionCrouch
  (params (Key :type Key%20Structure))
  (bind _charactermovement (Variables|Character|GetCharacterMovement))
  (:Pressed
    (if (not (Variables|Default|GetPronePressed))
      (Utilities|FlowControl|FlipFlop
        (:A
          (Variables|Default|SetCrouchPressed false)
          (if (Variables|Default|GetSprintPressed)
            _
            (else
              _))
          (Variables|/Script/Engine.CharacterMovementComponent|SetMaxWalkSpeed _charactermovement 0.0))
        (:B
          (Variables|Default|SetCrouchPressed false)
          (Variables|/Script/Engine.CharacterMovementComponent|SetMaxWalkSpeed _charactermovement 246.0))))))

(event Input|AxisEvents|InputAxisMoveForward
  (params (AxisValue :type Float%20%28single-precision%29))
  (if (not (Variables|Default|GetDisableMovement))
    (Pawn|Input|AddMovementInput (Math|Vector|GetForwardVector (Math|Rotator|MakeRotator 0.0 0.0 0.0)) AxisValue false)))

(event Input|AxisEvents|InputAxisStrafeRight
  (params (AxisValue :type Float%20%28single-precision%29))
  (if (not (Variables|Default|GetDisableMovement))
    (Pawn|Input|AddMovementInput (Math|Vector|GetRightVector (Math|Rotator|MakeRotator 0.0 0.0 0.0)) AxisValue false)))

(event Input|AxisEvents|InputAxisLookUp
  (params (AxisValue :type Float%20%28single-precision%29))
  (Pawn|Input|AddControllerPitchInput AxisValue))

(event Input|AxisEvents|InputAxisTurn
  (params (AxisValue :type Float%20%28single-precision%29))
  (Pawn|Input|AddControllerYawInput AxisValue))

(fn ConstructionScript)